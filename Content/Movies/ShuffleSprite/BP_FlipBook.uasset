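; Flipbook actor that plays a one-shot shuffle sprite animation with sound when its Activate event fires.
; Activate shows the PaperFlipbook, plays it from the start with the ShuffleV2 sound, and runs a timeline that drives the actor's uniform scale.
; Delays chained off the timeline's Update reverse the scale after two seconds, then hide the flipbook half a second later.
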(event Custom|Activate
  (Rendering|SetVisibility (Variables|Default|GetPaperFlipbook) true false)
  (Audio|PlaySound2D "/Game/Audio/ShuffleV2.ShuffleV2" 1.0 1.0 0.0 0 0)
  (Components|Timeline|PlayfromStart (Variables|Default|GetPaperFlipbook))
  (bind _scale (Timeline|Timeline Play)
    (:Update
      (Transformation|SetActorScale3D self (Math|Vector|MakeVector _scale _scale _scale))
      (Utilities|FlowControl|Delay 2.0)
      (Utilities|FlowControl|Sequence
        (:then_0
          (Timeline|Timeline Reverse))
        (:then_1
          (Utilities|FlowControl|Delay 0.5)
          (Rendering|SetVisibility (Variables|Default|GetPaperFlipbook) false false))))))

(event EventBeginPlay)

(fn ConstructionScript)