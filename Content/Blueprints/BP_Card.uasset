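; Card actor that animates its static mesh's yaw and has a scene capture component limited to rendering the card itself, set on BeginPlay.
; Roll and RollLeft each play their own timeline from the start to drive the mesh rotation.
; Reset reverses a third timeline, which nothing here plays forward, to write the yaw the same way.
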(event Custom|Roll
  (bind _newtrack_0 (Timeline|Timeline PlayFromStart)
    (:Update
      (Transformation|SetRelativeRotation (Variables|Default|GetStaticMesh) (Math|Rotator|MakeRotator 0.0 0.0 _newtrack_0) false false))))

(event Custom|RollLeft
  (bind _newtrack_0 (Timeline|Timeline_0 PlayFromStart)
    (:Update
      (Transformation|SetRelativeRotation (Variables|Default|GetStaticMesh) (Math|Rotator|MakeRotator 0.0 0.0 _newtrack_0) false false))))

(event Custom|Reset
  (bind _newtrack_0 (Timeline|Timeline_1 Reverse)
    (:Update
      (Transformation|SetRelativeRotation (Variables|Default|GetStaticMesh) (Math|Rotator|MakeRotator 0.0 0.0 _newtrack_0) false false))))

(event EventBeginPlay
  (Rendering|SceneCapture|ShowOnlyActorComponents (Variables|Default|GetSceneCaptureComponent2D) self false))

(fn ConstructionScript)