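; BP_Players is an actor that displays a player count using four components, Player1 through Player4, that share one material.
; UpdatePlayers shows as many components as the count given, hiding the rest along with their children, and UpdateColor applies a given material to all four.
; ResetNumber shows only Player1 without propagating to children, and FullReset also restores the grey material.
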(event Custom|UpdatePlayers
  (params (nbPlayers :type Integer))
  (switch int nbPlayers
    (:1
      (Rendering|SetVisibility (Variables|Default|GetPlayer%201) true true)
      (Rendering|SetVisibility (Variables|Default|GetPlayer%202) false true))
    (:2
      (Rendering|SetVisibility (Variables|Default|GetPlayer%201) true true)
      (Rendering|SetVisibility (Variables|Default|GetPlayer%203) false true))
    (:3
      (Rendering|SetVisibility (Variables|Default|GetPlayer%201) true true)
      (Rendering|SetVisibility (Variables|Default|GetPlayer%204) false true))
    (:4
      (Rendering|SetVisibility (Variables|Default|GetPlayer%201) true true))))

(event Custom|UpdateColor
  (params (NewParam :type Material%20Object%20Reference))
  (Rendering|Material|SetMaterial (Variables|Default|GetPlayer%201) 0 NewParam))

(event Custom|ResetNumber
  (Rendering|SetVisibility (Variables|Default|GetPlayer%201) true false)
  (Rendering|SetVisibility (Variables|Default|GetPlayer%202) false false))

(event Custom|FullReset
  (CallFunction|ResetNumber)
  (Rendering|Material|SetMaterial (Variables|Default|GetPlayer%201) 0 "/Game/Player/GREY.GREY"))

(event EventBeginPlay)

(event Collision|EventActorBeginOverlap
  (params (OtherActor :type Actor%20Object%20Reference)))

(event EventTick
  (params (DeltaSeconds :type Float%20%28single-precision%29)))

(fn ConstructionScript)