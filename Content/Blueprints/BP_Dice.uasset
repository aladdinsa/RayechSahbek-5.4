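; BP_Dice is a physics-driven die that rolls and reports which face lands up.
; ThrowDice randomizes height and pitch, plays a sound, applies a random sideways impulse, then evaluates the result and stops simulation after a fixed delay.
; Landed compares six face components' forward vectors to world up within a tolerance, writes a zero-based value to BP_GameInstance, then calls the DiceLanded dispatcher.
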(event Custom|ThrowDice
  (Transformation|SetRelativeLocation (Variables|Default|GetDice) (Math|Vector|MakeVector 0.0 0.0 (Math|Conversions|ToFloat(Integer) (Math|Random|RandomInteger 10))) true true)
  (Transformation|SetRelativeRotation (Variables|Default|GetDice) (Math|Rotator|MakeRotator 0.0 (Math|Conversions|ToFloat(Integer) (Math|Random|RandomInteger 360)) 0.0) false false)
  (Audio|PlaySound2D "/Game/Audio/DiceSFX.DiceSFX" 1.0 1.0 1.0 0 0)
  (Physics|SetSimulatePhysics (Variables|Default|GetDice) true)
  (Physics|AddImpulse (Variables|Default|GetDice) (Math|Vector|MakeVector 0.0 (Math|Conversions|ToFloat(Integer) (Math|Random|RandomIntegerinRange -800 -1000)) 0.0) "None" false)
  (Utilities|FlowControl|Delay 2.0)
  (CallFunction|Landed)
  (Physics|SetSimulatePhysics (Variables|Default|GetDice) false))

(event Custom|Landed
  (bind _as_bp_game_instance (Variables|Default|GetAs%20BP%20Game%20Instance))
  (Utilities|FlowControl|Sequence
    (:then_0
      (if (Utilities|Operators|EqualEqual (Math|Vector|GetForwardVector (Variables|Default|Get1)) "0.000000,0.000000,1.000000" 0.5)
        (Variables|/Game/Blueprints/BP_GameInstance.BP_GameInstance_C|SetCurrentDiceValue _as_bp_game_instance 0)))
    (:then_1
      (if (Utilities|Operators|EqualEqual (Math|Vector|GetForwardVector (Variables|Default|Get2)) "0.000000,0.000000,1.000000" 0.5)
        (Variables|/Game/Blueprints/BP_GameInstance.BP_GameInstance_C|SetCurrentDiceValue _as_bp_game_instance 1)))
    (:then_2
      (if (Utilities|Operators|EqualEqual (Math|Vector|GetForwardVector (Variables|Default|Get3)) "0.000000,0.000000,1.000000" 0.5)
        (Variables|/Game/Blueprints/BP_GameInstance.BP_GameInstance_C|SetCurrentDiceValue _as_bp_game_instance 2)))
    (:then_3
      (if (Utilities|Operators|EqualEqual (Math|Vector|GetForwardVector (Variables|Default|Get4)) "0.000000,0.000000,1.000000" 0.5)
        (Variables|/Game/Blueprints/BP_GameInstance.BP_GameInstance_C|SetCurrentDiceValue _as_bp_game_instance 3)))
    (:then_4
      (if (Utilities|Operators|EqualEqual (Math|Vector|GetForwardVector (Variables|Default|Get5)) "0.000000,0.000000,1.000000" 0.5)
        (Variables|/Game/Blueprints/BP_GameInstance.BP_GameInstance_C|SetCurrentDiceValue _as_bp_game_instance 4)))
    (:then_5
      (if (Utilities|Operators|EqualEqual (Math|Vector|GetForwardVector (Variables|Default|Get6)) "0.000000,0.000000,1.000000" 0.5)
        (Variables|/Game/Blueprints/BP_GameInstance.BP_GameInstance_C|SetCurrentDiceValue _as_bp_game_instance 5)))
    (:then_6
      (Default|CallDiceLanded))))

(event EventBeginPlay
  (bind _asbp_game_instance (Utilities|Casting|CastToBP_GameInstance (Game|GetGameInstance)))
  (Variables|Default|SetAs%20BP%20Game%20Instance _asbp_game_instance))

(fn ConstructionScript)

(fn Check)