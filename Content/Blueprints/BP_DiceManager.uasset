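; BP_DiceManager turns the dice value stored in BP_GameInstance into a question category and a random question from it.
; On Roll, it maps the value to the category, then gathers QuestionAR and ID from DT_Questions rows whose names contain that category's letter code, matched case-sensitively.
; One random index picks both question and ID, which it writes to the GameInstance before firing the RollTheDiceEvent dispatcher.
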(event Custom|Roll
  (CallFunction|RolltheDice)
  (Default|CallRolltheDiceEvent))

(event EventBeginPlay)

(event Collision|EventActorBeginOverlap
  (params (OtherActor :type Actor%20Object%20Reference)))

(event EventTick
  (params (DeltaSeconds :type Float%20%28single-precision%29)))

(fn ConstructionScript)

(fn RolltheDice
  (bind _questions (Variables|Default|GetQuestions))
  (Utilities|FlowControl|Sequence
    (:then_0
      (Utilities|Array|Clear (Variables|Default|GetQuestions))
      (bind _asbp_game_instance (Utilities|Casting|CastToBP_GameInstance (Game|GetGameInstance)))
      (Variables|Default|SetDiceValue (Variables|/Game/Blueprints/BP_GameInstance.BP_GameInstance_C|GetCurrentDiceValue _asbp_game_instance))
      (Variables|/Game/Blueprints/BP_GameInstance.BP_GameInstance_C|SetCurrentCategory _asbp_game_instance (Utilities|Select :Index (Variables|Default|GetDiceValue) :Option%200 "NewEnumerator0" :Option%201 "NewEnumerator1" :Option%202 "NewEnumerator2" :Option%203 "NewEnumerator3" :Option%204 "NewEnumerator4" :Option%205 "NewEnumerator5"))
      (bind _outrownames (DataTable|GetDataTableRowNames "/Game/Blueprints/DT_Questions.DT_Questions"))
      (for _array_element _outrownames
        (bind _returnvalue (Utilities|GetDataTableRow "/Game/Blueprints/DT_Questions.DT_Questions" _array_element)
          (:then
            (if (not (== (Utilities|String|FindSubstring (Utilities|String|ToString(Name) _array_element) (Utilities|Array|Get(acopy) (Variables|Default|GetCatLetters) (Variables|Default|GetDiceValue)) true) -1))
              (Utilities|FlowControl|Sequence
                (:then_0
                  (Utilities|Array|Add (Variables|Default|GetQuestions) (.QuestionAR (Utilities|Struct|BreakS_Question _returnvalue))))
                (:then_1
                  (Utilities|Array|Add (Variables|Default|GetQuestionIDs) (.QuestionID (Utilities|Struct|BreakS_Question _returnvalue)))))))))
      (bind _asbp_game_instance_2 (Utilities|Casting|CastToBP_GameInstance (Game|GetGameInstance)))
      (Variables|Default|SetRandomQuestionID (Math|Random|RandomInteger (Utilities|Array|Length _questions)))
      (Utilities|FlowControl|Sequence
        (:then_0
          (Variables|/Game/Blueprints/BP_GameInstance.BP_GameInstance_C|SetCurrentQuestion _asbp_game_instance_2 (Utilities|Array|Get(acopy) _questions (Variables|Default|GetRandomQuestionID))))
        (:then_1
          (Variables|/Game/Blueprints/BP_GameInstance.BP_GameInstance_C|SetCurrentQuestionID _asbp_game_instance_2 (Utilities|Array|Get(acopy) (Variables|Default|GetQuestionIDs) (Variables|Default|GetRandomQuestionID))))))
    (:then_1
      (Utilities|Array|Clear (Variables|Default|GetQuestionIDs)))))